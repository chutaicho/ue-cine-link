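; CineLink receiver Blueprint that drives a target camera actor's transform from incoming OSC messages.
; On BeginPlay it starts an OSC server listening on all interfaces at port 8000 and binds a message handler.
; The handler matches the camera transform address, unpacks the floats, and sets the valid TargetCamera's location and rotation.
; The first two position floats are swapped between X and Y, and values are applied directly without scaling or smoothing.
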(event `self.ReceiveBeginPlay`
  (bind _returnvalue (`OSCManager.CreateOSCServer` "0.0.0.0" 8000 false true "" null))
  (bind _output_get (set `self.OSCServer` _returnvalue))
  (add `OSCServer.OnOscMessageReceived` _output_get (delegate `HandleMessage`)))

(event `HandleMessage`
  (params (Message :type "OSCMessage Structure (by ref)") (IPAddress :type String) (Port :type Integer))
  (bind _targetcamera (`self.TargetCamera`))
  (bind _returnvalue (`OSCManager.GetOSCMessageAddress` Message))
  (bind _returnvalue_2 (`OSCManager.GetOSCAddressFullPath` _returnvalue))
  (switch `string` _returnvalue_2
    (:`/cinelink/cam/transform`
      (bind _values (`OSCManager.GetAllFloats` Message))
      (`/Engine/EditorBlueprintResources/StandardMacros.IsValid` _targetcamera
        (:`Is Valid`
          (`self.K2_SetActorLocationAndRotation` _targetcamera (`KismetMathLibrary.MakeVector` (`|GetArrayItem` _values 1) (`|GetArrayItem` _values) (`|GetArrayItem` _values 2)) (`KismetMathLibrary.MakeRotator` (`|GetArrayItem` _values 5) (`|GetArrayItem` _values 3) (`|GetArrayItem` _values 4)) false false))))))

(fn `UserConstructionScript`)