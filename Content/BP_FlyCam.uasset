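; Free-fly camera pawn driven by Enhanced Input.
; BeginPlay adds the IMC_FlyCam mapping context and caches the starting transform.
; Move actions feed movement input along actor forward, actor right and world up, while look drives controller yaw and pitch.
; Pan moves along the actor's right and up axes with horizontal inverted, and reset restores both the starting transform and control rotation.
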(event `self.ReceiveBeginPlay`
  (`EnhancedInputSubsystemInterface.AddMappingContext` (subsystem `EnhancedInputLocalPlayerSubsystem`) "/CineLink/Input/IMC_FlyCam.IMC_FlyCam" 0 (struct))
  (set `self.InitialLocation` (`self.K2_GetActorLocation`))
  (set `self.InitialRotation` (`self.K2_GetActorRotation`)))

(event `EnhancedInput|/CineLink/Input/IA_MoveForward`
  (params (ActionValue :type "Float (double-precision)") (ElapsedSeconds :type "Float (double-precision)") (TriggeredSeconds :type "Float (double-precision)") (InputAction :type "InputAction Object Reference" :default "/CineLink/Input/IA_MoveForward.IA_MoveForward"))
  (:`Triggered`
    (`self.AddMovementInput` (`self.GetActorForwardVector`) ActionValue)))

(event `EnhancedInput|/CineLink/Input/IA_MoveRight`
  (params (ActionValue :type "Float (double-precision)") (ElapsedSeconds :type "Float (double-precision)") (TriggeredSeconds :type "Float (double-precision)") (InputAction :type "InputAction Object Reference" :default "/CineLink/Input/IA_MoveRight.IA_MoveRight"))
  (:`Triggered`
    (`self.AddMovementInput` (`self.GetActorRightVector`) ActionValue)))

(event `EnhancedInput|/CineLink/Input/IA_MoveUp`
  (params (ActionValue :type "Float (double-precision)") (ElapsedSeconds :type "Float (double-precision)") (TriggeredSeconds :type "Float (double-precision)") (InputAction :type "InputAction Object Reference" :default "/CineLink/Input/IA_MoveUp.IA_MoveUp"))
  (:`Triggered`
    (`self.AddMovementInput` (`KismetMathLibrary.MakeVector` 0.0 0.0 1.0) ActionValue)))

(event `EnhancedInput|/CineLink/Input/IA_Look`
  (params (ActionValue :type "Vector2D Structure") (ElapsedSeconds :type "Float (double-precision)") (TriggeredSeconds :type "Float (double-precision)") (InputAction :type "InputAction Object Reference" :default "/CineLink/Input/IA_Look.IA_Look"))
  (bind (_x _y) (`KismetMathLibrary.BreakVector2D` ActionValue))
  (:`Triggered`
    (`self.AddControllerYawInput` _x)
    (`self.AddControllerPitchInput` _y)))

(event `EnhancedInput|/CineLink/Input/IA_Reset`
  (params (ActionValue :type Boolean) (ElapsedSeconds :type "Float (double-precision)") (TriggeredSeconds :type "Float (double-precision)") (InputAction :type "InputAction Object Reference" :default "/CineLink/Input/IA_Reset.IA_Reset"))
  (bind _initialrotation (`self.InitialRotation`))
  (:`Started`
    (`self.K2_SetActorLocationAndRotation` (`self.InitialLocation`) _initialrotation)
    (`Controller.SetControlRotation` (`self.GetController`) _initialrotation)))

(event `EnhancedInput|/CineLink/Input/IA_Pan`
  (params (ActionValue :type "Vector2D Structure") (ElapsedSeconds :type "Float (double-precision)") (TriggeredSeconds :type "Float (double-precision)") (InputAction :type "InputAction Object Reference" :default "/CineLink/Input/IA_Pan.IA_Pan"))
  (bind (_x _y) (`KismetMathLibrary.BreakVector2D` ActionValue))
  (:`Triggered`
    (`self.AddMovementInput` (`self.GetActorRightVector`) (* _x -1.0))
    (`self.AddMovementInput` (`self.GetActorUpVector`) _y)))

(fn `UserConstructionScript`)